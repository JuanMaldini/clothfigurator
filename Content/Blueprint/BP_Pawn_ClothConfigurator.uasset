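; Camera pawn for a cloth configurator that jumps between four preset views on a spring arm and cine camera.
; Events 1 to 4 call do-location, which resets the player controller's rotation, then applies that preset's root transform, arm length and focal length instantly.
; The construction script reapplies the stored Index.
; An unconnected branch would instead blend to tagged CineCameraActors.
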(event Custom|do-location
  (params (current-index :type String))
  (bind _returnvalue (Math|Conversions|ToInteger(Byte) current-index))
  (Utilities|FlowControl|Sequence
    (:then_0
      (bind _asbp_player_controller_cloth_configurator (Utilities|Casting|CastToBP_PlayerController_ClothConfigurator (Game|GetPlayerController 0)))
      (Default|Reset-rot _asbp_player_controller_cloth_configurator))
    (:then_1
      (Variables|Default|Sett-temp (Transformation|GetWorldTransform (Variables|Default|GetDefaultSceneRoot)))
      (Variables|Default|Sett-length (Variables|/Script/Engine.SpringArmComponent|GetTargetArmLength (Variables|Default|GetSpringArm)))
      (Variables|Default|Sett-currentFocalLength (Variables|/Script/CinematicCamera.CineCameraComponent|GetCurrentFocalLength (Variables|Default|GetCineCamera)))
      (Utilities|FlowControl|Sequence
        (:then_0
          (Transformation|SetWorldTransform (Variables|Default|GetDefaultSceneRoot) (Utilities|Select :Index _returnvalue :Option%200 (Variables|Default|Get1%20-%20Transform) :Option%201 (Variables|Default|Get2%20-%20Transform) :Option%202 (Variables|Default|Get3%20-%20Transform) :Option%203 (Variables|Default|Get4%20-%20Transform)) false false))
        (:then_1
          (Variables|/Script/Engine.SpringArmComponent|SetTargetArmLength (Variables|Default|GetSpringArm) (Utilities|Select :Index _returnvalue :Option%200 (Variables|Default|Get1%20-%20Length) :Option%201 (Variables|Default|Get2%20-%20Length) :Option%202 (Variables|Default|Get3%20-%20Length) :Option%203 (Variables|Default|Get4%20-%20Length))))
        (:then_2
          (Variables|/Script/CinematicCamera.CineCameraComponent|SetCurrentFocalLength (Variables|Default|GetCineCamera) (Utilities|Select :Index _returnvalue :Option%200 (Variables|Default|Get1%20-%20Focal%20Length) :Option%201 (Variables|Default|Get2%20-%20Focal%20Length) :Option%202 (Variables|Default|Get3%20-%20Focal%20Length) :Option%203 (Variables|Default|Get4%20-%20Focal%20Length))))
        (:then_3
          (Variables|Default|Setindex _returnvalue))))))

(event Custom|3
  (CallFunction|Do-location "2"))

(event Custom|1
  (CallFunction|Do-location "0"))

(event Custom|2
  (CallFunction|Do-location "1"))

(event Custom|4
  (CallFunction|Do-location "3"))

(fn ConstructionScript
  (CallFunction|Do-location (Utilities|String|ToString(Integer) (Variables|Default|Getindex))))