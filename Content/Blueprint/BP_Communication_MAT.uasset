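; Material manager Blueprint for a cloth configurator that applies fabric material instances to referenced static meshes, chosen by name or at random.
; On BeginPlay it fills MaterialList from the MayerFabrics folder through a recursive Asset Registry scan and caches the player controller.
; Set Material applies the pick to each SMRef mesh, using the map value as element index.
; The menu text printout is unwired and Refresh Material is empty.
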(event Custom|all-materials
  ;[0 0 0] ALL MATERIALS
  (CallFunction|Set-material (.OutItem (Utilities|Array|Random (Variables|Default|GetMaterial%20List)))))

(event Custom|set-material
  (params (Material :type Material%20Interface%20Object%20Reference))
  (bind _sm_ref (Variables|Default|GetSM%20ref))
  ;[0 0 0] SET MATERIAL
  (bind _keys (Utilities|Map|Keys _sm_ref))
  (for (_array_element _array_index) _keys
    (bind _values (Utilities|Map|Values _sm_ref))
    (Rendering|Material|SetMaterial (Variables|/Script/Engine.StaticMeshActor|GetStaticMeshComponent _array_element) (Utilities|Array|Get(acopy) _values _array_index) Material)))

(event Custom|refresh-material)

(event Custom|do-materials
  (params (material-name :type String))
  ;[0 0 0] DO MATERIALS
  (for _array_element (Variables|Default|GetMaterial%20List)
    (if (Utilities|Enum|Equal(Enum) (Utilities|GetObjectName _array_element) material-name)
      (bind _output_get (Variables|Default|Setmaterial-applied _array_element))
      (CallFunction|Set-material _output_get))))

(event Custom|collect_materials
  ;[0 0 0 0.5] COLLECT MATERIAL INSTANCES
  (CallFunction|Clear)
  (bind _outassetdata (Class|AssetRegistry|GetAssetsbyPath (Class|AssetRegistryHelpers|GetAssetRegistry) "/Game/Materials/MayerFabrics/" true false))
  (for _array_element _outassetdata
    (bind _asmaterial_instance (Utilities|Casting|CastToMaterialInstance (Class|AssetRegistryHelpers|GetAsset _array_element)))
    (Utilities|Array|AddUnique (Variables|Default|GetMaterial%20List) _asmaterial_instance)))

(event EventBeginPlay
  (CallFunction|CollectMaterials)
  (bind _asbp_player_controller_cloth_configurator (Utilities|Casting|CastToBP_PlayerController_ClothConfigurator (Game|GetPlayerController 0)))
  (Variables|Default|SetAs%20BP%20Player%20Controller%20Cloth%20Configurator _asbp_player_controller_cloth_configurator))

(fn ConstructionScript)

(fn Clear
  (Utilities|Array|Clear (Variables|Default|GetMaterial%20List))
  (return))