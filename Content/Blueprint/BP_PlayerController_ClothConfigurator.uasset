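; Player controller for a Pixel Streaming cloth configurator that fades in and applies a default tint, material and view on start.
; Frontend JSON events route to material changes via BP_Communication_MAT, tint via a material parameter collection, pawn camera views, or a screenshot sent back as a file.
; Mouse drag and touch rotate the Datasmith scene actor, a timeline event resets its rotation, and number keys switch views.
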(event Custom|reset-rot
  (bind _sda (Variables|Default|GetSDA))
  ;[0 0 0] RESET ROTATION
  (Variables|Default|Setrot1 (Transformation|GetActorRotation _sda))
  (bind _newtrack_0 (Timeline|Timeline PlayFromStart)
    (:Update
      (Transformation|SetActorRotation _sda (Math|Rotator|Lerp(Rotator) (Variables|Default|Getrot1) "0, 0, 0" _newtrack_0)))))

(event Custom|FadeStart
  (bind _returnvalue (Game|GetPlayerCameraManager 0))
  ;[0 0 0] MAKE FADE
  (Class|PlayerCameraManager|SetManualCameraFade :self _returnvalue :InFadeAmount 1.0)
  (Utilities|FlowControl|Delay 2.0)
  (CameraFades|StartCameraFade :self _returnvalue :FromAlpha 1.0 :Duration 1.0 :bHoldWhenFinished true))

(event Custom|FadeEnd
  (bind _returnvalue (Game|GetPlayerCameraManager 0))
  ;[0 0 0] MAKE FADE
  (Class|PlayerCameraManager|SetManualCameraFade :self _returnvalue)
  (Utilities|FlowControl|Delay 2.0)
  (CameraFades|StartCameraFade :self _returnvalue :ToAlpha 1.0 :Duration 1.0 :bHoldWhenFinished true))

(event Custom|UI%20Interaction
  (params (Descriptor :type String))
  (Variables|Default|SetDescriptor Descriptor)
  (CallFunction|UIInteractionEvent))

(event Custom|UI%20Interaction%20Event
  (bind _descriptor (Variables|Default|GetDescriptor))
  (bind _pixelstreaminginput (Variables|Default|GetPixelStreamingInput))
  (bind _descriptor_2 (Variables|Default|GetDescriptor))
  (bind _pixelstreaminginput_2 (Variables|Default|GetPixelStreamingInput))
  (bind _descriptor_3 (Variables|Default|GetDescriptor))
  (bind _pixelstreaminginput_3 (Variables|Default|GetPixelStreamingInput))
  (bind (_stringvalue _success) (Class|PixelStreamingInput|GetJsonStringValue _pixelstreaminginput _descriptor_3 "tint-change"))
  (bind (_stringvalue_2 _success_2) (Class|PixelStreamingInput|GetJsonStringValue _pixelstreaminginput_3 _descriptor "material-change"))
  (bind (_stringvalue_3 _success_3) (Class|PixelStreamingInput|GetJsonStringValue _pixelstreaminginput_2 _descriptor_2 "view"))
  ;[0 0 0] CHANGE MATERIAL
  (if _success_2
    (Default|Do-materials (Variables|Default|GetBPComm) _stringvalue_2)
    (else
      ;[0 0 0] CHANGE TINT
      (if _success
        (CallFunction|Do-tint _stringvalue)
        (else
          ;[0 0 0] TAKE AND DELIVER SCREENSHOT
          (if (.Success (Class|PixelStreamingInput|GetJsonStringValue (Variables|Default|GetPixelStreamingInput) (Variables|Default|GetDescriptor) "CreateScreenshot"))
            (CallFunction|Do-screenshot-PS)
            (else
              ;[0 0 0] SET VEW
              (if _success_3
                (Default|Do-location (Variables|Default|GetAs%20BP%20Pawn%20Cloth%20Configurator) _stringvalue_3)))))))))

(event Custom|Fake-PS-Event
  (params (Descriptor-Fake :type String))
  (Variables|Default|SetDescriptor Descriptor-Fake)
  (CallFunction|UIInteractionEvent))

(event Custom|do-screenshot-PS
  ;[0 0 0] Take Screenshot and send to the frontend (via send file)
  (Utilities|FlowControl|DoOnce false :!label _label
    (:Completed
      (Class|FileName|TakeScreenshot)
      (Utilities|FlowControl|Delay 0.3)
      (bind _returnvalue (Class|FileName|GetScreenshotFilePath))
      (Class|PixelStreamingBlueprints|SendFile _returnvalue "image/png" ".png")
      (Utilities|FlowControl|Delay 0.3)
      (Class|FileName|DeleteScreenshotFile _returnvalue)
      ;;[0 0 0] Send Json response back to frontend, to give a notice that this event was triggered and completed
      (Class|PixelStreamingInput|SendPixelStreamingResponse (Variables|Default|GetPixelStreamingInput) "CreateScreenshot")
      (goto _label Reset))))

(event EventBeginPlay
  (Utilities|FlowControl|Sequence
    (:then_0
      (for _array_element (Variables|Default|GetCommands)
        (Development|ExecuteConsoleCommand _array_element 0)))
    (:then_1
      (bind _returnvalue (Actor|GetActorOfClass "/Game/Blueprint/BP_Communication_MAT.BP_Communication_MAT_C"))
      (Variables|Default|SetBPComm _returnvalue))
    (:then_2
      (bind _asbp_pawn_cloth_configurator (Utilities|Casting|CastToBP_Pawn_ClothConfigurator (Game|Player|GetPlayerPawn 0)))
      (Variables|Default|SetAs%20BP%20Pawn%20Cloth%20Configurator _asbp_pawn_cloth_configurator))
    (:then_3
      (bind _returnvalue_2 (Actor|GetActorOfClass "/Script/DatasmithContent.DatasmithSceneActor"))
      (Variables|Default|SetSDA _returnvalue_2))
    (:then_4
      (EventDispatchers|BindEventtoOnInputEvent (Variables|Default|GetPixelStreamingInput) (delegate Custom|UI%20Interaction)))
    (:then_5
      (CallFunction|FadeStart))
    (:then_6
      (CallFunction|Fake-PS-Event "{\"tint-change\": \"R=1,G=1,B=1\"}")
      (CallFunction|Fake-PS-Event "{\"material-change\":\"MI_IMPACT_FUSE_BERRY-804-001\"}")
      (CallFunction|Fake-PS-Event "{\"view\":\"0\"}"))))

(event Input|MouseEvents|MouseX
  (params (AxisValue :type Float%20%28single-precision%29))
  ;[0 0 0] MOUSE IN X
  (if (Variables|Default|GetTouch_Hold)
    (Variables|Default|SetAxis%20Value AxisValue)
    (Class|Actor|AddActorWorldRotation (Variables|Default|GetSDA) (Math|Rotator|MakeRotator 0.0 0.0 (* (* (Variables|Default|GetAxis%20Value) -1.0) 6.0)))))

(event Input|KeyboardEvents|1
  (params (Key :type Key%20Structure :default "None"))
  ;[0.05 0 0] SET VIEWS
  (:Pressed
    (Default|Do-location (Variables|Default|GetAs%20BP%20Pawn%20Cloth%20Configurator) "0")))

(event Input|KeyboardEvents|2
  (params (Key :type Key%20Structure :default "None"))
  ;[0.05 0 0] SET VIEWS
  (:Pressed
    (Default|Do-location (Variables|Default|GetAs%20BP%20Pawn%20Cloth%20Configurator) "1")))

(event Input|KeyboardEvents|3
  (params (Key :type Key%20Structure :default "None"))
  ;[0.05 0 0] SET VIEWS
  (:Pressed
    (Default|Do-location (Variables|Default|GetAs%20BP%20Pawn%20Cloth%20Configurator) "2")))

(event Input|KeyboardEvents|4
  (params (Key :type Key%20Structure :default "None"))
  ;[0.05 0 0] SET VIEWS
  (:Pressed
    (Default|Do-location (Variables|Default|GetAs%20BP%20Pawn%20Cloth%20Configurator) "3")))

(event Input|MouseEvents|LeftMouseButton
  (params (Key :type Key%20Structure :default "None"))
  (:Pressed
    (Variables|/Script/Engine.PlayerController|SetbShowMouseCursor (Game|GetPlayerController 0) true)
    (Variables|Default|SetIs_Tactil false)
    (Variables|Default|SetTouch_Hold true))
  (:Released
    (Variables|Default|SetTouch_Hold false)))

(event Input|MouseEvents|RightMouseButton
  (params (Key :type Key%20Structure :default "None"))
  (:Pressed
    (Variables|/Script/Engine.PlayerController|SetbShowMouseCursor (Game|GetPlayerController 0) true)
    (Variables|Default|SetIs_Tactil false)
    (Variables|Default|SetTouch_Hold true))
  (:Released
    (Variables|Default|SetTouch_Hold false)))

(event Input|TouchEvents|InputTouch
  (params (Location :type Vector) (FingerIndex :type ETouchIndex%20Enum))
  (bind _returnvalue (Game|GetPlayerController 0))
  (bind (_locationx _locationy) (Class|PlayerController|GetInputTouchState _returnvalue "Touch1"))
  (:Pressed
    (Variables|Default|Settouch-loc-last-1 Location)
    (Utilities|FlowControl|Sequence
      (:then_0
        (Variables|/Script/Engine.PlayerController|SetbShowMouseCursor (Game|GetPlayerController 0) false)
        (Variables|Default|SetIs_Tactil true))
      (:then_1
        (Variables|Default|SetTouch_Hold true)
        (Variables|Default|SetTouch_Location_Previous (Math|Vector2D|MakeVector2D _locationx _locationy) :!label _label))))
  (:Released
    (Variables|Default|Settouch-loc-last-1 Location)
    (Utilities|FlowControl|Sequence
      (:then_0
        (if (Variables|Default|GetTouch_Hold)
          (Variables|Default|SetTouch_Hold false)))
      (:then_1
        (goto _label))))
  (:Moved
    (Class|Actor|AddActorWorldRotation (Variables|Default|GetSDA) (Math|Rotator|MakeRotator 0.0 0.0 (* (.X (Math|Vector|BreakVector (- (Variables|Default|Gettouch-loc-last-1) Location))) 0.25)))
    (Variables|Default|Settouch-loc-last-1 Location)))

(fn ConstructionScript)

(fn TouchRotation
  (params (Location_X :type Float%20%28double-precision%29) (Location_Y :type Float%20%28double-precision%29))
  (Variables|Default|SetTouch_Location_Current (Math|Vector2D|MakeVector2D Location_X Location_Y))
  (Development|PrintString (Utilities|String|ToString(Float) (+ (* (- (/ (.x (Variables|Default|GetTouch_Location_Current)) (.x (Variables|Default|GetTouch_Location_Previous))) 1.0) 1e+02) (.yaw (Pawn|GetControlRotation :!class /Script/Engine.Controller)))))
  (Variables|Default|SetTouch_Location_Previous (Math|Vector2D|MakeVector2D (.x (Variables|Default|GetTouch_Location_Current)) (.y (Variables|Default|GetTouch_Location_Current)))))

(fn Do-tint
  (params (RGB :type String))
  (Rendering|Material|SetVectorParameterValue "/Game/FabricCollection/Materials/MasterMaterials/UtilityFunctions/MPC_ColorTintPS.MPC_ColorTintPS" "color-tint" (.OutConvertedColor (Math|Conversions|ToColor(LinearColor) RGB)) :!class /Script/Engine.KismetMaterialLibrary))